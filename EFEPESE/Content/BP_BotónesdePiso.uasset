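; BP_BotónesdePiso is a floor-button code puzzle that opens a linked Door when the player steps on the buttons in the correct order.
; The Construction Script spawns a row of flattened meshes spaced along X, each with an overlap box tagged with one character of RandomCode.
; First-person character overlaps append that tag to InputCode.
; At CorrectCode's length, a match sends OpenDoorMessage to Door, otherwise the input resets.
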(event EventBeginPlay)

(event Collision|EventActorBeginOverlap
  (params (OtherActor :type Actor%20Object%20Reference)))

(event EventTick
  (params (DeltaSeconds :type Float%20%28single-precision%29)))

(fn ConstructionScript
  (for _index (range 0 (- (Utilities|String|Len (Variables|Default|GetCorrectCode)) 1))
    (bind _returnvalue (AddComponent|AddStaticMeshComponent false (Math|Transform|MakeTransform (Math|Vector|MakeVector (* _index (Variables|Default|GetSpacing)) 0.0 0.0) "0, 0, 0" "1.000000,1.000000,0.100000")))
    (bind _returnvalue_2 (AddComponent|AddBoxComponent false (Math|Transform|MakeTransform (+ (Variables|/Script/Engine.SceneComponent|GetRelativeLocation _returnvalue) "50.000000,50.000000,50.000000") "0, 0, 0" "1.000000,1.000000,1.000000")))
    (Variables|/Script/Engine.ActorComponent|SetComponentTags _returnvalue_2 (Utilities|Array|MakeArray (Utilities|String|StringToName (Utilities|String|GetSubstring (Variables|Default|GetRandomCode) _index))))
    (Collision|BindEventtoOnComponentBeginOverlap _returnvalue_2 (EventDispatchers|CreateEvent :!event BPBotónesdePisoAutoGenFunc))))

(fn BPBotónesdePisoAutoGenFunc
  (params (OverlappedComponent :type Primitive%20Component%20Object%20Reference) (OtherActor :type Actor%20Object%20Reference) (OtherComp :type Primitive%20Component%20Object%20Reference) (OtherBodyIndex :type Integer) (bFromSweep :type Boolean) (SweepResult :type Hit%20Result%20Structure%20%28by%20ref%29))
  (Utilities|Casting|CastToBP_FirstPersonCharacter OtherActor)
  (CallFunction|AñadirAlCodigo (Utilities|String|ToString(Name) (Utilities|Array|Get(acopy) (Variables|/Script/Engine.ActorComponent|GetComponentTags OverlappedComponent))))
  (return))

(fn AñadirAlCodigo
  (params (Añadir :type String))
  (Variables|Default|SetInputCode (Utilities|String|Append (Variables|Default|GetInputCode) Añadir))
  (if (== (Utilities|String|Len (Variables|Default|GetInputCode)) (Utilities|String|Len (Variables|Default|GetCorrectCode)))
    (if (Utilities|Enum|Equal(Enum) (Variables|Default|GetCorrectCode) (Variables|Default|GetInputCode))
      (Class|PuzzleInterface|OpenDoor(Message) (Variables|Default|GetDoor))
      (else
        (Variables|Default|SetInputCode "")))))